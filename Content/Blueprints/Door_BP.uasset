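; Keycard-locked sliding door that rises while a player who can open it overlaps the actor and lowers after they leave.
; On overlap, a locked door unlocks if the BucksAlgCharacter holds at least one keycard, then sets MoveObject.
; Tick moves the mesh vertically in fixed, frame-rate-dependent steps between its start height and roughly one mesh height above.
; SetIsLocked also swaps the material, but the overlap unlock bypasses it.
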(event EventBeginPlay
  (Variables|Default|SetStartLocation (Transformation|GetWorldLocation (Variables|Default|GetStaticMesh)))
  (Variables|Default|SetMoveObject false))

(event Collision|EventActorBeginOverlap
  (params (OtherActor :type Actor%20Object%20Reference))
  (if (Pawn|IsPlayerControlled (Variables|/Script/Engine.Actor|GetInstigator OtherActor))
    (Utilities|FlowControl|Sequence
      (:then_0
        (if (not (Variables|Default|GetisUnlocked))
          (bind _asbucks_alg_character (Utilities|Casting|CastToBucksAlgCharacter OtherActor))
          (bind _returnvalue (Class|BucksAlgCharacter|GetKeycardAmount _asbucks_alg_character))
          (Variables|Default|SetisUnlocked (>= _returnvalue 1))))
      (:then_1
        (if (Variables|Default|GetisUnlocked)
          (Variables|Default|SetMoveObject true))))))

(event EventTick
  (params (DeltaSeconds :type Float%20%28single-precision%29))
  (if (Variables|Default|GetMoveObject)
    (Utilities|MoveUp)
    (else
      (Utilities|MoveDown))))

(event Collision|EventActorEndOverlap
  (params (OtherActor :type Actor%20Object%20Reference))
  (if (Pawn|IsPlayerControlled (Variables|/Script/Engine.Actor|GetInstigator OtherActor))
    (Variables|Default|SetMoveObject false)))

(fn ConstructionScript)

(fn SetIsLocked
  (params (IsUnlocked :type Boolean))
  (bind _output_get (Variables|Default|SetisUnlocked IsUnlocked))
  (if _output_get
    (Rendering|Material|SetMaterial (Variables|Default|GetStaticMesh) 0 "/Game/StarterContent/Props/Materials/M_Door.M_Door")
    (else
      (Rendering|Material|SetMaterial (Variables|Default|GetStaticMesh) 0 "/Game/StarterContent/Materials/M_Wood_Oak.M_Wood_Oak"))))